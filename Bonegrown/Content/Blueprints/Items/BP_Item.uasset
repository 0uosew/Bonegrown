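; BP_Item is a pickup that grants a power-up when a BP_ShooterCharacter overlaps its sphere.
; The construction script sets the static mesh and material from the Item variable.
; On overlap it fetches the BP_FirstPersonCharacter by class rather than using the overlapping actor, passes ItemType to PowerUps, plays the item's tooltip through that character's UI_Manager, then destroys itself.
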(event OnComponentBeginOverlap(Sphere)
  (params (OverlappedComponent :type Primitive%20Component%20Object%20Reference) (OtherActor :type Actor%20Object%20Reference) (OtherComp :type Primitive%20Component%20Object%20Reference) (OtherBodyIndex :type Integer) (bFromSweep :type Boolean) (SweepResult :type Hit%20Result%20Structure%20%28by%20ref%29))
  (if (== (Utilities|GetClass OtherActor) "/Game/Variant_Shooter/Blueprints/BP_ShooterCharacter.BP_ShooterCharacter_C")
    (bind _returnvalue (Actor|GetActorOfClass "/Game/FirstPerson/Blueprints/BP_FirstPersonCharacter.BP_FirstPersonCharacter_C"))
    (Default|PowerUps _returnvalue (Variables|Default|GetItemType))
    (Default|PlayTooltip (Actor|GetComponentbyClass _returnvalue "/Game/Blueprints/UI_Manager.UI_Manager_C") (Variables|Default|GetItem))
    (Actor|DestroyActor)))

(fn ConstructionScript
  (bind _item (Variables|Default|GetItem))
  (bind _staticmesh (Variables|Default|GetStaticMesh))
  (bind (_name _thumbnail _isstackable _mesh _material) (Utilities|Struct|BreakS_ItemStruct _item))
  (Components|StaticMesh|SetStaticMesh _staticmesh _mesh)
  (Rendering|Material|SetMaterial _staticmesh 0 _material))