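; BP_ItemBase is a pickup item, apparently a base for item types, that grants power-ups to the player.
; On sphere overlap, it casts to BP_ShooterCharacter and has the character check the overlapping component.
; It then passes ItemType to AddPowerUps, sends name, description and thumbnail to the UI_Manager tooltip, and destroys itself.
; MakeMatGlow sets a dynamic emissive material parameter, but nothing here runs it.
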(event OnComponentBeginOverlap(Sphere)
  (params (OverlappedComponent :type Primitive%20Component%20Object%20Reference) (OtherActor :type Actor%20Object%20Reference) (OtherComp :type Primitive%20Component%20Object%20Reference) (OtherBodyIndex :type Integer) (bFromSweep :type Boolean) (SweepResult :type Hit%20Result%20Structure%20%28by%20ref%29))
  ;[0.15 0.15 0.15 0.5] When Touched Sends Item Data to Player and UI Manager
  ;;[0.15 0.005739 0.000781 0.5] Might Hurt Performance / Casting Every Pickup
  (bind _asbp_shooter_character (Utilities|Casting|CastToBP_ShooterCharacter OtherActor))
  (bind _output_get (Variables|Default|SetAs%20BP%20Shooter%20Character _asbp_shooter_character))
  (if (|Checksifothercompisplayer_2 (Variables|Default|GetAs%20BP%20Shooter%20Character) OtherComp)
    (Default|AddPowerUps _output_get (Variables|Default|GetItemType))
    (Default|PlayTooltip (Actor|GetComponentbyClass (Variables|Default|GetAs%20BP%20Shooter%20Character) "/Game/Blueprints/UI_Manager.UI_Manager_C") (Variables|Default|GetItemName) (Variables|Default|GetItemDescription) (Variables|Default|GetItemThumbnail))
    (Actor|DestroyActor)))

(fn ConstructionScript)

(fn MakeMatGlow
  (bind _staticmesh (Variables|Default|GetStaticMesh))
  (bind _returnvalue (Rendering|Material|CreateDynamicMaterialInstance _staticmesh 0 (Rendering|Material|GetMaterial _staticmesh 0) "None" :!class /Script/Engine.PrimitiveComponent))
  (bind _output_get (Variables|Default|SetDynamic%20Emissive%20Material _returnvalue))
  (Rendering|Material|SetMaterial _staticmesh 0 (Variables|Default|GetDynamic%20Emissive%20Material))
  (Class|MaterialInstanceDynamic|SetScalarParameterbyIndex _output_get 0 1.0))