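; BP_ItemBase is a pickup item that grants the player a power-up on touch.
; When its Sphere overlaps the capsule of BP_ShooterCharacter, it passes ItemType to that character's AddPowerUp.
; It then shows the item's name, description and thumbnail through the UI_Manager component on BP_FirstPersonCharacter, and destroys itself.
; Both characters are found with GetActorOfClass; the construction script and NewFunction are empty.
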(event OnComponentBeginOverlap(Sphere)
  (params (OverlappedComponent :type Primitive%20Component%20Object%20Reference) (OtherActor :type Actor%20Object%20Reference) (OtherComp :type Primitive%20Component%20Object%20Reference) (OtherBodyIndex :type Integer) (bFromSweep :type Boolean) (SweepResult :type Hit%20Result%20Structure%20%28by%20ref%29))
  (bind _returnvalue (Actor|GetActorOfClass "/Game/Variant_Shooter/Blueprints/BP_ShooterCharacter.BP_ShooterCharacter_C"))
  (if (== OtherComp (Variables|/Script/Engine.Character|GetCapsuleComponent _returnvalue))
    (bind _returnvalue_2 (Actor|GetActorOfClass "/Game/FirstPerson/Blueprints/BP_FirstPersonCharacter.BP_FirstPersonCharacter_C"))
    (bind _returnvalue_3 (Actor|GetActorOfClass "/Game/Variant_Shooter/Blueprints/BP_ShooterCharacter.BP_ShooterCharacter_C"))
    (Default|AddPowerUp _returnvalue_3 (Variables|Default|GetItemType))
    (Default|PlayTooltip (Actor|GetComponentbyClass _returnvalue_2 "/Game/Blueprints/UI_Manager.UI_Manager_C") (Variables|Default|GetItemName) (Variables|Default|GetItemDescription) (Variables|Default|GetItemThumbnail))
    (Actor|DestroyActor)))

(fn ConstructionScript)

(fn NewFunction)