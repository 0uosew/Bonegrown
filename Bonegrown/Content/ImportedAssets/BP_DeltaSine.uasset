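; Actor component that bobs its owning actor vertically along a sine wave, set by Speed and Strength.
; Each tick advances a time counter and moves the owner to InitLoc plus the Z offset, optionally using the absolute value for a bouncing motion.
; On BeginPlay, RandomizePeriod gives a random starting phase; InitLoc is captured only in that same branch.
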(event EventBeginPlay
  ;[1 1 1] Randomize Period?
  (if (Variables|Default|GetRandomize%20Period)
    (Variables|Default|SetTime (* (Math|Random|RandomFloat) 5e+02))
    (Variables|Default|SetInitLoc (Transformation|GetActorLocation (Components|GetOwner)))))

(event EventTick
  (params (DeltaSeconds :type Float%20%28single-precision%29))
  (bind _returnvalue (Components|GetOwner))
  (bind _initloc (Variables|Default|GetInitLoc))
  (bind _output_get (Variables|Default|SetTime (+ (Variables|Default|GetTime) (* DeltaSeconds 1e+02))))
  (bind _output_get_2 (Variables|Default|SetWave (* (Math|Trig|Sin(Degrees) (* _output_get (Variables|Default|GetSpeed))) (Variables|Default|GetStrength))))
  (if (Variables|Default|GetAbs)
    (Transformation|SetActorLocation _returnvalue (+ _initloc (Math|Vector|MakeVector 0.0 0.0 (Math|Float|Absolute(Float) _output_get_2))) false false)
    (else
      (Transformation|SetActorLocation _returnvalue (+ _initloc (Math|Vector|MakeVector 0.0 0.0 _output_get_2)) false false))))