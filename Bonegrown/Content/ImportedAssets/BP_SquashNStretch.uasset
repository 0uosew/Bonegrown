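; BP_SquashNStretch is a component that gives its owning actor a looping squash-and-stretch animation.
; Each tick it advances a time value and sets the owner's scale from a sine wave scaled by Strength, moving X and Z in opposite directions around one while Y stays fixed.
; An optional RandomizePeriod flag randomizes the starting time on BeginPlay, offsetting the phase between instances.
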(event EventBeginPlay
  (if (Variables|Default|GetRandomize%20Period)
    (Variables|Default|SetTime (* (Math|Random|RandomFloat) 5e+02))))

(event EventTick
  (params (DeltaSeconds :type Float%20%28single-precision%29))
  (bind _output_get (Variables|Default|SetTime (+ (Variables|Default|GetTime) (* DeltaSeconds 1e+02))))
  (bind _output_get_2 (Variables|Default|SetWave (* (Math|Trig|Sin(Degrees) _output_get) (Variables|Default|GetStrength))))
  (Transformation|SetActorScale3D (Components|GetOwner) (Math|Vector|MakeVector (+ (* _output_get_2 -1.0) 1.0) 1.0 (+ _output_get_2 1.0))))